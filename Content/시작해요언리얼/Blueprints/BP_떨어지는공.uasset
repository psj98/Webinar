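; BP_떨어지는공 (falling ball) is a trap that drops a ball when BP_ThirdPersonCharacter triggers it and fails the player on contact.
; Actor overlap reveals the sphere and enables physics on it and its collision sphere.
; Tick polls the collision sphere for player overlap and calls CollisionSphere, which ragdolls the player, disables input and shows the failure result widget.
; No one-shot guard exists, so continued overlap can create repeated widgets.
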(event Collision|EventActorBeginOverlap
  (params (OtherActor :type Actor%20Object%20Reference))
  (Utilities|Casting|CastToBP_ThirdPersonCharacter OtherActor)
  (Physics|SetSimulatePhysics (Variables|Default|GetSphere) true)
  (Physics|SetSimulatePhysics (Variables|Default|GetSphereCollision) true)
  (Development|SetHiddeninGame (Variables|Default|GetSphere) false false))

(event EventTick
  (params (DeltaSeconds :type Float%20%28single-precision%29))
  (bind _asbp_third_person_character (Utilities|Casting|CastToBP_ThirdPersonCharacter (Game|GetPlayerCharacter 0)))
  (if (Collision|IsOverlappingActor (Variables|Default|GetSphereCollision) _asbp_third_person_character :!class /Script/Engine.PrimitiveComponent)
    (CallFunction|CollisionSphere)))

(fn ConstructionScript)

(fn CollisionSphere
  (bind _returnvalue (Game|GetPlayerCharacter 0))
  (bind _mesh (Variables|/Script/Engine.Character|GetMesh _returnvalue))
  (Utilities|IsValid _returnvalue
    (:Is%20Valid
      (Collision|SetCollisionEnabled (Variables|/Script/Engine.Character|GetCapsuleComponent _returnvalue) "NoCollision")
      (Pawn|Components|CharacterMovement|SetMovementMode (Variables|/Script/Engine.Character|GetCharacterMovement _returnvalue) "MOVE_None" 0)
      (Collision|SetCollisionProfileName _mesh "Ragdoll" true :!class /Script/Engine.PrimitiveComponent)
      (Class|SkeletalMeshComponent|SetAllBodiesSimulatePhysics _mesh true)
      (EventDispatchers|UnbindallEventsfromOnActorBeginOverlap (Game|GetPlayerCharacter 0))
      (bind _returnvalue_2 (UserInterface|CreateWidget "/Game/시작해요언리얼/Blueprints/BP_결과화면위젯.BP_결과화면위젯_C" (Game|GetPlayerController 0))) ; 결과화면 위젯 표시
      (Utilities|FlowControl|Sequence
        (:then_0
          (UserInterface|Viewport|AddtoViewport _returnvalue_2 0) ; 화면에 표시
        )
        (:then_1
          (Input|DisableInput (Game|GetPlayerCharacter 0) (Game|GetPlayerController 0))
          (Input|SetInputModeUIOnly (Game|GetPlayerController 0) _returnvalue_2 "DoNotLock"))
        (:then_2
          (Default|SetResult _returnvalue_2 false))))))